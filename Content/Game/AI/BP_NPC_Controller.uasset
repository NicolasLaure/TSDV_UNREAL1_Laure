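; BP_NPC_Controller is the controller that drives an NPC car along a track spline.
; On BeginPlay it casts its pawn to BP_AI_Car, calls Init with the car's track spline and sets acceleration, distance, car width and steering tuning values.
; Each Tick it feeds TickAI's steering, throttle and brake outputs to the car, scaling throttle down.
; Init and TickAI are defined outside this graph.
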(event `self.ReceiveBeginPlay`
  (bind _asbp_ai_car (cast `/Game/Game/AI/BP_AI_Car` (`self.K2_GetPawn`)))
  (set `self.BpCar` _asbp_ai_car)
  (`self.Init` (`/Game/Game/Scripts/BP_TrackSpline.Spline` (`/Game/Game/AI/BP_AI_Car.Track` _asbp_ai_car)))
  (set `self.accelThreshold` 0.65)
  (set `self.minDistance` 75.0)
  (set `self.carWidth` 400.0)
  (set `self.steeringForce` 0.8))

(event `self.ReceiveTick`
  (params (DeltaSeconds :type "Float (single-precision)"))
  (bind _bpcar (`self.BpCar`))
  (bind (_accel _brake _steering) (`self.TickAI`))
  (`/Game/Game/AI/BP_AI_Car.Steering` _bpcar _steering)
  (`/Game/Game/AI/BP_AI_Car.Throttle` _bpcar (* _accel 0.6))
  (`/Game/Game/AI/BP_AI_Car.Brake` _bpcar _brake))

(fn `UserConstructionScript`)