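; Runs the rules of a timed checkpoint race, from start countdown to win or lose screen.
; BeginPlay binds checkpoint events and disables car input, then GameStart restores input and starts the time limit and lap clock.
; Checkpoints extend remaining time and broadcast their transform.
; A finish crossing counts only when one checkpoint remains visible, then either resets checkpoints for the next lap or wins, pausing the game.
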(event `self.ReceiveBeginPlay`
  (`GameplayStatics.SetGamePaused` false)
  (`|ExecutionSequence`
    (:`then_0`
      (bind _outactors (`GameplayStatics.GetAllActorsOfClass` "/Game/Game/Scripts/BP_CheckPointBP.BP_CheckPointBP_C"))
      (for _array_element _outactors
        (if (`/Game/Game/Scripts/BP_CheckPointBP.IsFinishLine` _array_element)
          (add `/Game/Game/Scripts/BP_CheckPointBP.OnFinishLineCrossed` _array_element (`|CreateDelegate` :!event `OnFinishLineCrossed`))
          (else
            (add `/Game/Game/Scripts/BP_CheckPointBP.OnCheckPointCrossed` _array_element (delegate `HandleCheckPointCrossed`))))))
    (:`then_1`
      (`self.StartCountdown`)
      (bind _asbp_mclaren (cast `/Game/Assets/Cars/Mclaren/BP_Mclaren` (`GameplayStatics.GetPlayerPawn` 0)))
      (`self.DisableInput` _asbp_mclaren null))))

(event `HandleCheckPointCrossed`
  (params (Position :type "Vector Structure") (Rotation :type "Rotator Structure"))
  (`|ExecutionSequence`
    (:`then_0`
      (`self.OnLastCheckPointChanged` Position Rotation))
    (:`then_1`
      (`KismetSystemLibrary.PrintString` "CrossedCheckPoint")
      (`self.StartTimerEvent` (+ (`KismetSystemLibrary.K2_GetTimerRemainingTimeHandle` (`self.Time Remaining`)) (`self.CheckPointReward`))))))

(event `FinishInitialCountDown`
  (`self.GameStart`))

(event `StartCountdown`
  (`KismetSystemLibrary.PrintString` "CountDown Started")
  (bind _returnvalue (`KismetSystemLibrary.K2_SetTimerDelegate` (delegate `FinishInitialCountDown`) (`self.StartDelay`)))
  (set `self.InitialTimer` _returnvalue))

(event `GameStart`
  (bind _returnvalue (`GameplayStatics.GetPlayerController` 0))
  (bind _asbp_player_controller (cast `/Game/Game/Player/BP_PlayerController` _returnvalue))
  (`/Game/Game/Player/BP_PlayerController.OnDisableInput` _asbp_player_controller)
  (`self.StartTimerEvent` (`self.Start Timer Duration`))
  (bind _asbp_player_controller_2 (cast `/Game/Game/Player/BP_PlayerController` _returnvalue))
  (`/Game/Game/Player/BP_PlayerController.OnEnableInput` _asbp_player_controller_2 "/Game/Game/Player/PlayerInput.PlayerInput")
  (`KismetSystemLibrary.K2_SetTimerDelegate` (`|CreateDelegate` :!event `IncreaseTime`) 0.001 true))

(event `Lose`
  (`self.GameFinish` false))

(event `IncreaseTime`
  (bind (_remainder _returnvalue) (`KismetMathLibrary.FMod` (/ (`self.LapTotalMs`) 1000.0) 60.0))
  (bind _returnvalue_2 (`KismetMathLibrary.FTrunc` _remainder))
  (`/Engine/EditorBlueprintResources/StandardMacros.IncrementFloat` (`self.LapTotalMs`)
    (:`  `
      (set `self.LapMinutes` _returnvalue)
      (set `self.LapSeconds` _returnvalue_2)
      (set `self.LapMs` (`KismetMathLibrary.FTrunc` (* (- _remainder _returnvalue_2) 1000.0))))))

(event `GameFinish`
  (params (Win :type Boolean))
  (`GameplayStatics.SetGamePaused` true)
  (bind _asuser_widget (castclass `UserWidget` (`KismetMathLibrary.SelectClass` "/Game/Hud/WBP_Win.WBP_Win_C" "/Game/Hud/WBP_Lose.WBP_Lose_C" Win)))
  (bind _returnvalue (`|CreateWidget` _asuser_widget))
  (`UserWidget.AddToViewport` _returnvalue 0))

(event `Win`
  (`KismetSystemLibrary.K2_ClearAndInvalidateTimerHandle` (`self.Time Remaining`))
  (`self.GameFinish` true))

(event `OnFinishLineCrossed`
  (bind _currentlap (`self.currentLap`))
  (bind _outactors (`GameplayStatics.GetAllActorsOfClass` "/Game/Game/Scripts/BP_CheckPointBP.BP_CheckPointBP_C"))
  (set `self.ActiveCheckPoints` 0)
  (for _array_element _outactors
    (if (== (`/Game/Game/Scripts/BP_CheckPointBP.IsHidden` _array_element) false)
      (set `self.ActiveCheckPoints` (+ (`self.ActiveCheckPoints`) 1))))
  (if (== (`self.ActiveCheckPoints`) 1)
    (if (== _currentlap (`self.MaxLaps`))
      (`self.Win`)
      (else
        (set `self.currentLap` (+ _currentlap 1))
        (bind _outactors_2 (`GameplayStatics.GetAllActorsOfClass` "/Game/Game/Scripts/BP_CheckPointBP.BP_CheckPointBP_C"))
        (for _array_element_2 _outactors_2
          (`/Game/Game/Scripts/BP_CheckPointBP.OnReset` _array_element_2))))))

(event `StartTimerEvent`
  (params (TimerDuration :type "Float (double-precision)"))
  (`KismetSystemLibrary.PrintString` (`KismetStringLibrary.Concat_StrStr` "Timer Started with Duration: " (`KismetStringLibrary.Conv_DoubleToString` TimerDuration)))
  (bind _returnvalue (`KismetSystemLibrary.K2_SetTimerDelegate` (`|CreateDelegate` :!event `Lose`) TimerDuration))
  (set `self.Time Remaining` _returnvalue))

(fn `UserConstructionScript`)