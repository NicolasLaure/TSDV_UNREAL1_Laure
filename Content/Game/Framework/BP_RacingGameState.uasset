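; BP_RacingGameState is a racing game state Blueprint that tracks lap time as minutes, seconds and milliseconds.
; Each OnTimeIncrease event increments TimeInMs by one, with no timer or caller in this graph.
; It converts that count to seconds and splits it with whole-and-remainder division into LapMinutes, LapSeconds and LapMs, truncating the remainder for seconds and scaling its fraction for milliseconds.
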(event `OnTimeIncrease`
  (bind _result (`/Engine/EditorBlueprintResources/StandardMacros.IncrementFloat` (`self.TimeInMs`))
    (:`  `
      (bind (_remainder _returnvalue) (`KismetMathLibrary.FMod` (/ _result 1000.0) 60.0))
      (set `self.LapMinutes` _returnvalue)
      (bind _returnvalue_2 (`KismetMathLibrary.FTrunc` _remainder))
      (set `self.LapSeconds` _returnvalue_2)
      (set `self.LapMs` (`KismetMathLibrary.FTrunc` (* (- _remainder _returnvalue_2) 1000.0))))))

(fn `UserConstructionScript`)