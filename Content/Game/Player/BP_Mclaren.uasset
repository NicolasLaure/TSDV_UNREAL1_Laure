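; Player-drivable McLaren Chaos vehicle for a racing game, with spring-arm mouse camera, checkpoint respawn and pit stops.
; Driving inputs feed the movement component and call WheelDegradation on the affected wheels, weighted by input type; tire changes restore them.
; It stores checkpoint transforms from BP_RacingGame's dispatcher for position restarts.
; Pit entry hides the car and disables input; exit teleports it to BP_PitLaneExit and restores both.
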(event `Mouse X`
  (params (AxisValue :type "Float (double-precision)"))
  ;[1 1 1] Camera
  (`SceneComponent.K2_AddRelativeRotation` (`self.SpringArm`) (`KismetMathLibrary.MakeRotator` 0.0 0.0 AxisValue) false false))

(event `Mouse Y`
  (params (AxisValue :type "Float (double-precision)"))
  ;[1 1 1] Camera
  (`SceneComponent.K2_AddRelativeRotation` (`self.SpringArm`) (`KismetMathLibrary.MakeRotator` 0.0 AxisValue) false false))

(event `Throttle`
  (params (`Axis Value` :type "Float (double-precision)"))
  (bind _wheeldegradation (`self.WheelDegradation`))
  (bind _wheelcomponent (`self.WheelComponent`))
  (`ChaosVehicleMovementComponent.SetThrottleInput` (`self.VehicleMovementComponent`) `Axis Value`)
  (`/Game/Game/Player/BP_WheelDegradation.DegradeWheel` _wheeldegradation "RL" _wheelcomponent 1.0 :!label _label)
  (`/Game/Game/Player/BP_WheelDegradation.DegradeWheel` _wheeldegradation "RR" _wheelcomponent 1.0))

(event `self.ReceiveBeginPlay`
  (`|ExecutionSequence`
    (:`then_0`
      (set `self.LastCheckPointRotation` (`self.K2_GetActorRotation`))
      (set `self.LastCheckPointPosition` (`self.K2_GetActorLocation`))
      (bind _returnvalue (`GameplayStatics.GetActorOfClass` "/Game/Game/Scripts/BP_PitLaneExit.BP_PitLaneExit_C"))
      (set `self.PitLaneExit` _returnvalue)
      (bind _aschaos_wheeled_vehicle_movement_component (cast `ChaosWheeledVehicleMovementComponent` (`self.VehicleMovementComponent`)))
      (set `self.WheelComponent` _aschaos_wheeled_vehicle_movement_component))
    (:`then_1`
      (bind _asbp_racing_game (cast `/Game/Game/Framework/BP_RacingGame` (`GameplayStatics.GetGameMode`)))
      (add `/Game/Game/Framework/BP_RacingGame.OnLastCheckPointChanged` _asbp_racing_game (`|CreateDelegate` :!event `OnLastCheckPointUpdated`)))))

(event `Brake`
  (params (`Axis Value` :type "Float (double-precision)"))
  (bind _wheeldegradation (`self.WheelDegradation`))
  (bind _wheelcomponent (`self.WheelComponent`))
  (`ChaosVehicleMovementComponent.SetBrakeInput` (`self.VehicleMovementComponent`) `Axis Value`)
  (`/Game/Game/Player/BP_WheelDegradation.DegradeWheel` _wheeldegradation "FL" _wheelcomponent 6.0 :!label _label_2)
  (`/Game/Game/Player/BP_WheelDegradation.DegradeWheel` _wheeldegradation "FR" _wheelcomponent 6.0))

(event `HandBrakePress`
  (`ChaosVehicleMovementComponent.SetHandbrakeInput` (`self.VehicleMovementComponent`) true)
  (`|ExecutionSequence`
    (:`then_0`
      (goto _label))
    (:`then_1`
      (goto _label_2))))

(event `HandBrakeRelease`
  (`ChaosVehicleMovementComponent.SetHandbrakeInput` (`self.VehicleMovementComponent`) false))

(event `Steering`
  (params (NewParam :type "Float (double-precision)"))
  (bind _wheeldegradation (`self.WheelDegradation`))
  (bind _wheelcomponent (`self.WheelComponent`))
  (`ChaosVehicleMovementComponent.SetSteeringInput` (`self.VehicleMovementComponent`) NewParam)
  (if (!= NewParam 0.0)
    (if (< NewParam 0.0)
      (`/Game/Game/Player/BP_WheelDegradation.DegradeWheel` _wheeldegradation "FR" _wheelcomponent 3.0)
      (`/Game/Game/Player/BP_WheelDegradation.DegradeWheel` _wheeldegradation "RR" _wheelcomponent 3.0)
      (else
        (`/Game/Game/Player/BP_WheelDegradation.DegradeWheel` _wheeldegradation "FL" _wheelcomponent 3.0)
        (`/Game/Game/Player/BP_WheelDegradation.DegradeWheel` _wheeldegradation "RL" _wheelcomponent 3.0)))))

(event `RestartPosition`
  (bind _lastcheckpointrotation (`self.LastCheckPointRotation`))
  (`self.K2_SetActorRotation` _lastcheckpointrotation)
  (`self.K2_TeleportTo` (+ (`self.LastCheckPointPosition`) (0.0 0.0 20.0)) _lastcheckpointrotation)
  (`Controller.SetControlRotation` (`self.GetController` (`GameplayStatics.GetPlayerPawn` 0)) _lastcheckpointrotation)
  (`ChaosVehicleMovementComponent.ResetVehicle` (`self.VehicleMovementComponent`)))

(event `OnLastCheckPointUpdated`
  (params (Position :type "Vector Structure") (Rotation :type "Rotator Structure"))
  (`|ExecutionSequence`
    (:`then_0`
      (`KismetSystemLibrary.PrintString` "Setting Last CheckPoint")
      (set `self.LastCheckPointPosition` Position))
    (:`then_1`
      (bind _output_get (set `self.LastCheckPointRotation` Rotation))
      (`KismetSystemLibrary.PrintString` (`KismetStringLibrary.Conv_RotatorToString` _output_get)))))

(event `OnPitEntryTrigger`
  (`self.OnPitEntry`)
  (`self.SetActorHiddenInGame` true)
  (`self.DisableInput` (`GameplayStatics.GetPlayerController` 0)))

(event `OnPitExit`
  (bind _rotation (.rotation (`self.GetTransform` (`self.PitLaneExit`))))
  (`self.EnableInput` (`GameplayStatics.GetPlayerController` 0))
  (`ChaosVehicleMovementComponent.ResetVehicle` (`self.VehicleMovementComponent`))
  (`self.K2_TeleportTo` (.location (`self.GetTransform` (`self.PitLaneExit`))) _rotation)
  (`self.SetActorHiddenInGame` false)
  (`Controller.SetControlRotation` (`self.GetController`) _rotation))

(event `OnTiresChanged`
  (bind _aschaos_wheeled_vehicle_movement_component (cast `ChaosWheeledVehicleMovementComponent` (`self.VehicleMovementComponent`)))
  (`/Game/Game/Player/BP_WheelDegradation.RestoreWheels` (`self.WheelDegradation`) _aschaos_wheeled_vehicle_movement_component))

(fn `UserConstructionScript`)