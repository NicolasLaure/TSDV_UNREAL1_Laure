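; Player controller that relays Enhanced Input driving, camera and restart actions to the player's BP_Mclaren car.
; BeginPlay casts and caches player pawn 0 as the Mclaren reference that receives every input call.
; Throttle, brake and steering forward their value on both Triggered and Completed, while the handbrake maps to press and release calls.
; An IsActive flag, toggled by OnEnableInput and OnDisableInput, gates all actions.
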(event `EnhancedInput|/Game/Game/Player/Actions/Throttle`
  (params (ActionValue :type "Float (double-precision)") (ElapsedSeconds :type "Float (double-precision)") (TriggeredSeconds :type "Float (double-precision)") (InputAction :type "InputAction Object Reference" :default "/Game/Game/Player/Actions/Throttle.Throttle"))
  (bind _isactive (`self.IsActive`))
  (:`Triggered`
    (if _isactive
      (`/Game/Assets/Cars/Mclaren/BP_Mclaren.Throttle` (`self.Mclaren`) ActionValue :!label _label)))
  (:`Completed`
    (if _isactive
      (goto _label))))

(event `EnhancedInput|/Game/Game/Player/Actions/Brake`
  (params (ActionValue :type "Float (double-precision)") (ElapsedSeconds :type "Float (double-precision)") (TriggeredSeconds :type "Float (double-precision)") (InputAction :type "InputAction Object Reference" :default "/Game/Game/Player/Actions/Brake.Brake"))
  (bind _isactive (`self.IsActive`))
  (:`Triggered`
    (if _isactive
      (`/Game/Assets/Cars/Mclaren/BP_Mclaren.Brake` (`self.Mclaren`) ActionValue :!label _label_2)))
  (:`Completed`
    (if _isactive
      (goto _label_2))))

(event `EnhancedInput|/Game/Game/Player/Actions/Steering`
  (params (ActionValue :type "Float (double-precision)") (ElapsedSeconds :type "Float (double-precision)") (TriggeredSeconds :type "Float (double-precision)") (InputAction :type "InputAction Object Reference" :default "/Game/Game/Player/Actions/Steering.Steering"))
  (bind _isactive (`self.IsActive`))
  (:`Triggered`
    (if _isactive
      (`/Game/Assets/Cars/Mclaren/BP_Mclaren.Steering` (`self.Mclaren`) ActionValue :!label _label_3)))
  (:`Completed`
    (if _isactive
      (goto _label_3))))

(event `EnhancedInput|/Game/Game/Player/Actions/HandBrake`
  (params (ActionValue :type Boolean) (ElapsedSeconds :type "Float (double-precision)") (TriggeredSeconds :type "Float (double-precision)") (InputAction :type "InputAction Object Reference" :default "/Game/Game/Player/Actions/HandBrake.HandBrake"))
  (bind _mclaren (`self.Mclaren`))
  (bind _isactive (`self.IsActive`))
  (:`Triggered`
    (if _isactive
      (`/Game/Assets/Cars/Mclaren/BP_Mclaren.HandBrakePress` _mclaren)))
  (:`Completed`
    (if _isactive
      (`/Game/Assets/Cars/Mclaren/BP_Mclaren.HandBrakeRelease` _mclaren))))

(event `self.ReceiveBeginPlay`
  (bind _asbp_mclaren (cast `/Game/Assets/Cars/Mclaren/BP_Mclaren` (`GameplayStatics.GetPlayerPawn` 0)))
  (set `self.Mclaren` _asbp_mclaren))

(event `EnhancedInput|/Game/Game/Player/Actions/Restart`
  (params (ActionValue :type Boolean) (ElapsedSeconds :type "Float (double-precision)") (TriggeredSeconds :type "Float (double-precision)") (InputAction :type "InputAction Object Reference" :default "/Game/Game/Player/Actions/Restart.Restart"))
  (:`Started`
    (if (`self.IsActive`)
      (`/Game/Assets/Cars/Mclaren/BP_Mclaren.RestartPosition` (`self.Mclaren`)))))

(event `OnDisableInput`
  (set `self.IsActive` false))

(event `EnhancedInput|/Game/Game/Player/Actions/Camera`
  (params (ActionValue :type "Vector2D Structure") (ElapsedSeconds :type "Float (double-precision)") (TriggeredSeconds :type "Float (double-precision)") (InputAction :type "InputAction Object Reference" :default "/Game/Game/Player/Actions/Camera.Camera"))
  (bind (_x _y) (`KismetMathLibrary.BreakVector2D` ActionValue))
  (bind _mclaren (`self.Mclaren`))
  (:`Triggered`
    (if (`self.IsActive`)
      (`/Game/Assets/Cars/Mclaren/BP_Mclaren.Mouse X` _mclaren _x)
      (`/Game/Assets/Cars/Mclaren/BP_Mclaren.Mouse Y` _mclaren _y))))

(event `OnEnableInput`
  (params (Mapping :type "InputMappingContext Object Reference"))
  (set `self.IsActive` true))

(fn `UserConstructionScript`)