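; BP_WheelDegradation tracks wear on four vehicle wheels and turns it into reduced tire performance.
; DegradeWheel lowers the named wheel's value by a scaled rate, then SetWheelDegradation lerps that clamped value into slip and friction multipliers on the wheeled component.
; Rear wheels use their own maximum grip.
; RestoreWheels resets all four values, but its mismatched order applies FR and RL before they are reset.
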(fn `DegradeWheel`
  (params (WheelToDegrade :type String) (WheelComponent :type "ChaosWheeledVehicleMovementComponent Object Reference") (Multiplier :type "Float (double-precision)"))
  (bind _returnvalue (* (`self.DegradationRate`) Multiplier))
  (switch `string` WheelToDegrade
    (:`FL`
      (set `self.FL` (- (`self.FL`) _returnvalue)))
    (:`FR`
      (set `self.FR` (- (`self.FR`) _returnvalue)))
    (:`RL`
      (set `self.RL` (- (`self.RL`) _returnvalue)))
    (:`RR`
      (set `self.RR` (- (`self.RR`) _returnvalue))))
  (`self.SetWheelDegradation` WheelToDegrade WheelComponent))

(fn `RestoreWheels`
  (params (WheeledVehicle :type "ChaosWheeledVehicleMovementComponent Object Reference"))
  (bind _maxwheel (`self.MaxWheel`))
  (set `self.FL` _maxwheel)
  (`self.SetWheelDegradation` "FL" WheeledVehicle)
  (set `self.RR` _maxwheel)
  (`self.SetWheelDegradation` "FR" WheeledVehicle)
  (set `self.FR` _maxwheel)
  (`self.SetWheelDegradation` "RL" WheeledVehicle)
  (set `self.RL` _maxwheel)
  (`self.SetWheelDegradation` "RR" WheeledVehicle))

(fn `SetWheelDegradation`
  (params (Name :type String) (WheeledComponent :type "ChaosWheeledVehicleMovementComponent Object Reference"))
  (locals (Aux :type "Float (double-precision)") (wheelIndex :type Integer) (AuxMaxGrip :type "Float (double-precision)"))
  (bind _wheeled_component (`self.Wheeled Component`))
  (bind _wheelindex (`local.wheelIndex`))
  (bind _maxreargrip (`self.MaxRearGrip`))
  (bind _returnvalue (`KismetMathLibrary.FClamp` (`local.Aux`)))
  (set `self.Wheeled Component` WheeledComponent)
  (set `local.wheelIndex` 0)
  (set `local.AuxMaxGrip` (`self.MaxGrip`))
  (set `local.Aux` 0.0)
  (switch `string` Name
    (:`FL`
      (set `local.Aux` (`self.FL`))
      (set `local.wheelIndex` 0))
    (:`FR`
      (set `local.Aux` (`self.FR`))
      (set `local.wheelIndex` 1))
    (:`RL`
      (set `local.Aux` (`self.RL`))
      (set `local.AuxMaxGrip` _maxreargrip)
      (set `local.wheelIndex` 2))
    (:`RR`
      (set `local.Aux` (`self.RR`))
      (set `local.AuxMaxGrip` _maxreargrip)
      (set `local.wheelIndex` 3)))
  (`ChaosWheeledVehicleMovementComponent.SetWheelSlipGraphMultiplier` _wheeled_component _wheelindex (`KismetMathLibrary.Lerp` (`self.MinSlip`) (`self.MaxSlip`) _returnvalue))
  (`ChaosWheeledVehicleMovementComponent.SetWheelFrictionMultiplier` _wheeled_component _wheelindex (`KismetMathLibrary.Lerp` (`self.MinGrip`) (`local.AuxMaxGrip`) _returnvalue)))