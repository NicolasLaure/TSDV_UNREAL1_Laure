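; BP_CheckPointBP is a race checkpoint that can also act as the finish line, triggered when a BP_Mclaren overlaps its CheckPoint collision component.
; As a finish line it broadcasts OnFinishLineCrossed and stays active.
; Otherwise it broadcasts OnCheckPointCrossed with its location and rotation, then hides itself and disables collision.
; OnReset makes it visible again and restores query and physics collision.
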(event `OnReset`
  (bind _output_get (set `self.IsHidden` false))
  (`self.SetActorHiddenInGame` _output_get)
  (`PrimitiveComponent.SetCollisionEnabled` (`self.CheckPoint`) "QueryAndPhysics"))

(event `self.CheckPoint.OnComponentBeginOverlap`
  (params (OverlappedComponent :type "PrimitiveComponent Object Reference") (OtherActor :type "Actor Object Reference") (OtherComp :type "PrimitiveComponent Object Reference") (OtherBodyIndex :type Integer) (bFromSweep :type Boolean) (SweepResult :type "HitResult Structure (by ref)"))
  (cast `/Game/Game/Player/BP_Mclaren` OtherActor)
  (if (`self.IsFinishLine`)
    (`self.OnFinishLineCrossed`)
    (else
      (`self.OnCheckPointCrossed` (`self.K2_GetActorLocation`) (`self.K2_GetActorRotation`))
      (bind _output_get (set `self.IsHidden` true))
      (`self.SetActorHiddenInGame` _output_get)
      (`PrimitiveComponent.SetCollisionEnabled` (`self.CheckPoint`) "NoCollision"))))

(fn `UserConstructionScript`)